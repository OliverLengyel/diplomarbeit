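; Base HUD that draws the crosshair, five-slot quick bar, minimap image and a cursor-position debug readout, plus the inventory screen while the character is in input mode.
; DrawInventory lays out slots from the character's inventory array, adding hit boxes named by index for hover highlighting and drag pickup.
; Clicking empties the slot and draws the item at the cursor; releasing over a hit box calls the character's inventory update.
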(event `self.ReceiveHitBoxBeginCursorOver`
  (params (BoxName :type Name))
  ;[1 1 1] Mouse over events
  (if (`PlayerController.IsLookInputIgnored` (`GameplayStatics.GetPlayerController` 0))
    (set `self.Hit Box Name` BoxName)
    (set `self.MouseIsHoveringOverHitBox` true)
    (set `self.HitBoxHighlighted` (`KismetStringLibrary.Conv_StringToInt` (`KismetStringLibrary.Conv_NameToString` BoxName)))))

(event `self.ReceiveHitBoxEndCursorOver`
  (params (BoxName :type Name))
  ;[1 1 1] Mouse over events
  (if (`PlayerController.IsLookInputIgnored` (`GameplayStatics.GetPlayerController` 0))
    (set `self.MouseIsHoveringOverHitBox` false)))

(event `self.ReceiveHitBoxClick`
  (params (BoxName :type Name))
  ;[1 1 1] Mouse over events
  (if (`PlayerController.IsLookInputIgnored` (`GameplayStatics.GetPlayerController` 0))
    (set `self.ItemPickedUp` true)
    (set `self.HitBox To Int` (`KismetStringLibrary.Conv_StringToInt` (`KismetStringLibrary.Conv_NameToString` (stale `self.ReceiveHitBoxBeginCursorOver` BoxName))))
    (`self.ItemMousePickup`)
    (`/Engine/EditorBlueprintResources/StandardMacros.Gate` true :!label _label)))

(event `self.ReceiveTick`
  (params (DeltaSeconds :type "Float (single-precision)"))
  ;[1 1 1] Mouse over events
  (goto _label :!via `Open`))

(event `self.ReceiveHitBoxRelease`
  (params (BoxName :type Name))
  ;[1 1 1] Mouse over events
  (if (`PlayerController.IsLookInputIgnored` (`GameplayStatics.GetPlayerController` 0))
    (set `self.ItemPickedUp` false)
    (`self.ButtonReleased`)
    (goto _label :!via `Close`)))

(event `self.ReceiveDrawHUD`
  (params (SizeX :type Integer) (SizeY :type Integer))
  (bind (_x _y) (`KismetMathLibrary.BreakVector2D` (`self.ScreenDimension`)))
  ;[1 1 1] determine screen size
  (set `self.ScreenDimension` (`KismetMathLibrary.MakeVector2D` (`KismetMathLibrary.Conv_IntToDouble` SizeX) (`KismetMathLibrary.Conv_IntToDouble` SizeY)))
  (`|ExecutionSequence`
    (:`then_0`
      ;[1 1 1] Draw crosshair
      (`self.DrawTexture` (`self.crosshair`) (- (/ _x 2.0) 15.0) (- (/ _y 2.0) 15.0) 30.0 30.0 0.0 0.0 1.0 1.0 (struct :`R` 1.0 :`G` 1.0 :`B` 1.0 :`A` 1.0) "BLEND_Masked" 1.0 false 0.0 (0.0 0.0))
      (`self.Draw Quick Bar`))
    (:`then_1`
      (bind _asbase_character_bp_c (cast `/Game/Blueprints/Characters/Base_Character_BP` (`GameplayStatics.GetPlayerCharacter` 0)))
      (if (`/Game/Blueprints/Characters/Base_Character_BP.Is Input Mode` _asbase_character_bp_c)
        (`self.Draw Inventory`)
        (`self.TextureUpdateViaPickUp`)
        ;[1 1 1] adjust Inventory Hud
        (for (_ _array_index) (`/Game/Blueprints/Characters/Base_Character_BP.CharacterInventory` _asbase_character_bp_c)
          (if (and (== (`self.Hit Box Name`) (`KismetStringLibrary.Conv_StringToName` (`KismetStringLibrary.Conv_IntToString` _array_index))) (`self.MouseIsHoveringOverHitBox`))
            (bind _scale_out (`self.ScaledBasedOnIndex` _array_index))
            (bind (_x_2 _y_2) (`KismetMathLibrary.BreakVector2D` (`KismetArrayLibrary.Array_Get` (`self.Hit Box Position`) _array_index)))
            (`self.DrawTextureSimple` "/Game/Blueprints/Hud/HotBarButtonPressed.HotBarButtonPressed" _x_2 _y_2 _scale_out)
            (if (>= _array_index (`self.Inventory slots`))
              (`self.DrawText` (`KismetStringLibrary.Conv_IntToString` (- _array_index (- (`self.Inventory slots`) 1))) (struct) (+ _x_2 5.0) _y_2))))))
    (:`then_2`
      ;[1 1 1] MiniMap
      (`self.DrawTexture` "/Game/Blueprints/Hud/MiniMap.MiniMap" 0.0 475.0 256.0 256.0 0.0 0.0 1.0 1.0 (struct :`R` 1.0 :`G` 1.0 :`B` 1.0 :`A` 1.0) "BLEND_Opaque"))))

(fn `Button Highlighted`
  (params (`HitBox Name` :type Name))
  (switch `name` `HitBox Name`
    (:`Quick Slot 1`
      (set `self.QuickBtn1 Pressed` true)
      (set `self.ItemHighlightedToArray` 50))
    (:`Quick Slot 2`
      (set `self.QuickBtn2 Pressed` true)
      (set `self.ItemHighlightedToArray` 51))
    (:`Quick Slot 3`
      (set `self.QuickBtn3 Pressed` true)
      (set `self.ItemHighlightedToArray` 52))
    (:`Quick Slot 4`
      (set `self.QuickBtn4 Pressed` true)
      (set `self.ItemHighlightedToArray` 53))
    (:`Quick Slot 5`
      (set `self.QuickBtn5 Pressed` true)
      (set `self.ItemHighlightedToArray` 54))))

(fn `Button Unhighlighted`
  (params (`Hit Box Name` :type Name))
  (switch `name` `Hit Box Name`
    (:`Quick Slot 1`
      (set `self.QuickBtn1 Pressed` false))
    (:`Quick Slot 2`
      (set `self.QuickBtn2 Pressed` false))
    (:`Quick Slot 3`
      (set `self.QuickBtn3 Pressed` false))
    (:`Quick Slot 4`
      (set `self.QuickBtn4 Pressed` false))
    (:`Quick Slot 5`
      (set `self.QuickBtn5 Pressed` false))))

(fn `ButtonReleased`
  (if (`self.MouseIsHoveringOverHitBox`)
    (bind _asbase_character_bp_c (cast `/Game/Blueprints/Characters/Base_Character_BP` (`self.GetOwningPawn`)))
    (`/Game/Blueprints/Characters/Base_Character_BP.UpdateinventoryItemsViaHud` _asbase_character_bp_c)))

(fn `Draw Inventory`
  (bind (_x _y) (`KismetMathLibrary.BreakVector2D` (`self.ScreenDimension`)))
  (bind (_x_2 _y_2) (`KismetMathLibrary.BreakVector2D` (`self.ScreenDimension`)))
  (bind (_x_3 _y_3) (`KismetMathLibrary.BreakVector2D` (`self.ScreenDimension`)))
  (bind _returnvalue (/ _y_2 1.108))
  (bind _returnvalue_2 (+ (* (- (`self.CurrentInventoryIndex`) (`self.CurrentColumn`)) (`self.QuickBarArrayIncreaserX`)) (- _x_2 1108.0)))
  (bind _returnvalue_3 (`KismetMathLibrary.MakeVector2D` (+ (* (- (`self.CurrentInventoryIndex`) (`self.CurrentColumn`)) (`self.Inventory Array IncreaserX`)) (- _x_3 512.0)) (+ (/ _y_3 2.0) (`self.Inventory Array IncreaserY`))))
  (bind _returnvalue_4 (`KismetMathLibrary.MakeVector2D` _returnvalue_2 _returnvalue))
  ;[1 1 1] render equipment
  (`self.DrawTextureSimple` "/Game/Blueprints/Hud/UI_elements.UI_elements")
  ;[1 1 1] render inventory slots
  (`self.DrawTextureSimple` "/Game/Blueprints/Hud/inventory_background.inventory_background" (- _x 517.5) (/ _y 2.02))
  (bind _asbase_character_bp_c (cast `/Game/Blueprints/Characters/Base_Character_BP` (`self.GetOwningPawn`)))
  (for (_array_element _array_index) (`/Game/Blueprints/Characters/Base_Character_BP.CharacterInventory` _asbase_character_bp_c)
    (set `self.CurrentInventoryIndex` _array_index)
    ;[1 1 1] inventory menu funkyness
    (set `self.CurrentInventoryArrayElement` _array_element)
    (if (== (mod (`self.CurrentInventoryIndex`) (`self.InventoryModulusMath`)) 0)
      (set `self.CurrentColumn` (`self.CurrentInventoryIndex`))
      (if (>= (`self.CurrentInventoryIndex`) (`self.Inventory slots`))
        (`self.AddHitBox` (84.0 84.0) _returnvalue_4 (`KismetStringLibrary.Conv_StringToName` (`KismetStringLibrary.Conv_IntToString` (`self.CurrentInventoryIndex`))) :!label _label)
        (`KismetArrayLibrary.Array_Add` (`self.Hit Box Position`) _returnvalue_4)
        (`/Engine/EditorBlueprintResources/StandardMacros.IsValid` _array_element
          (:`Is Valid`
            (`self.DrawTextureSimple` (`/Game/Blueprints/Pickups/BaseItemPlaceHolder.ItemInventoryTexture` _array_element) _returnvalue_2 _returnvalue 0.9)))
        (else
          (set `self.Inventory Array IncreaserY` (* (`self.CurrentInventoryIndex`) 5.11))
          (`self.AddHitBox` _returnvalue_3 (50.0 50.0) (`KismetStringLibrary.Conv_StringToName` (`KismetStringLibrary.Conv_IntToString` (`self.CurrentInventoryIndex`))) :!label _label_2)
          (`KismetArrayLibrary.Array_Add` (`self.Hit Box Position`) _returnvalue_3)
          (`/Engine/EditorBlueprintResources/StandardMacros.IsValid` _array_element)))
      (elif (>= (`self.CurrentInventoryIndex`) (`self.Inventory slots`))
        (goto _label)
        (else
          (goto _label_2))))))

(fn `Draw Quick Bar`
  (bind (_locationx _locationy) (`PlayerController.GetMousePosition` (`GameplayStatics.GetPlayerController` 0)))
  ;[1 1 1] quick slot 1
  (bind (_output_x _output_y _outscale) (`self.ScaleToRatio` 420.0 (`self.QuickSlot Y Location`) (`self.Scale`)))
  (`self.DrawTextureSimple` (`self.Button Unpressed`) _output_x _output_y _outscale)
  (`self.DrawText` "1" (`self.Text Colour`) (+ _output_x 5.0) _output_y)
  (bind (_output_x_2 _output_y_2 _outscale_2) (`self.ScaleToRatio` 510.0 (`self.QuickSlot Y Location`) (`self.Scale`)))
  (`self.DrawTextureSimple` (`self.Button Unpressed`) _output_x_2 _output_y_2 _outscale_2)
  (`self.DrawText` "2" (`self.Text Colour`) (+ _output_x_2 5.0) _output_y_2)
  ;[1 1 1] quick slot 3
  (bind (_output_x_3 _output_y_3 _outscale_3) (`self.ScaleToRatio` 600.0 (`self.QuickSlot Y Location`) (`self.Scale`)))
  (`self.DrawTextureSimple` (`self.Button Unpressed`) _output_x_3 _output_y_3 _outscale_3)
  (`self.DrawText` "3" (`self.Text Colour`) (+ _output_x_3 5.0) _output_y_3)
  (bind (_output_x_4 _output_y_4 _outscale_4) (`self.ScaleToRatio` 690.0 (`self.QuickSlot Y Location`) (`self.Scale`)))
  (`self.DrawTextureSimple` (`self.Button Unpressed`) _output_x_4 _output_y_4 _outscale_4)
  (`self.DrawText` "4" (`self.Text Colour`) (+ _output_x_4 5.0) _output_y_4)
  ;[1 1 1] quick slot 5
  (bind (_output_x_5 _output_y_5 _outscale_5) (`self.ScaleToRatio` 780.0 (`self.QuickSlot Y Location`) (`self.Scale`)))
  (`self.DrawTextureSimple` (`self.Button Unpressed`) _output_x_5 _output_y_5 _outscale_5)
  (`self.DrawText` "5" (`self.Text Colour`) (+ _output_x_5 5.0) _output_y_5)
  ;[1 1 1] Cursor location debug feature
  (`self.DrawText` (`KismetStringLibrary.Concat_StrStr` (`KismetStringLibrary.Concat_StrStr` (`KismetStringLibrary.Conv_DoubleToString` _locationx) "X ") (`KismetStringLibrary.Concat_StrStr` (`KismetStringLibrary.Conv_DoubleToString` _locationy) "Y ")) (struct :`R` 1.0 :`G` 1.0 :`B` 1.0 :`A` 1.0)))

(fn `ItemMousePickup`
  (set `self.Store Index` (`self.HitBox To Int`))
  (bind _asbase_character_bp_c (cast `/Game/Blueprints/Characters/Base_Character_BP` (`GameplayStatics.GetPlayerCharacter` 0)))
  (bind _characterinventory (`/Game/Blueprints/Characters/Base_Character_BP.CharacterInventory` _asbase_character_bp_c))
  (set `self.Item Being Moved` (`KismetArrayLibrary.Array_Get` _characterinventory (`self.HitBox To Int`)))
  (`KismetArrayLibrary.Array_Set` _characterinventory (`self.HitBox To Int`)))

(fn `ScaledBasedOnIndex`
  (params (Index :type Integer))
  (returns (`Scale Out` :type "Float (double-precision)"))
  (if (>= Index 50)
    (set `self.Scale Out Variable` 1.7)
    (else
      (set `self.Scale Out Variable` 1.0)))
  (return (`self.Scale Out Variable`)))

(fn `ScaleToRatio`
  (params (`Input X` :type "Float (double-precision)") (`Input Y` :type "Float (double-precision)") (InScale :type "Float (double-precision)"))
  (returns (`Output X` :type "Float (double-precision)") (`Output Y` :type "Float (double-precision)") (OutScale :type "Float (double-precision)"))
  (bind (_sizex _sizey) (`PlayerController.GetViewportSize` (`GameplayStatics.GetPlayerController` 0)))
  (bind (_x _y) (`KismetMathLibrary.BreakVector2D` (`self.ScreenDimension`)))
  (set `self.ScreenDimension` (`KismetMathLibrary.MakeVector2D` (`KismetMathLibrary.Conv_IntToDouble` _sizex) (`KismetMathLibrary.Conv_IntToDouble` _sizey)))
  (`|ExecutionSequence`
    (:`then_0`
      (set `self.RatioX` (/ _x (`self.Screen Resolution X`))))
    (:`then_1`
      (set `self.RatioY` (/ _y (`self.Screen Resolution Y`))))
    (:`then_2`
      (return (* `Input X` (`self.RatioX`)) (* `Input Y` (`self.RatioY`)) (* InScale (`self.RatioY`))))))

(fn `TextureUpdateViaPickUp`
  (bind (_locationx _locationy) (`PlayerController.GetMousePosition` (`GameplayStatics.GetPlayerController` 0)))
  (if (`self.ItemPickedUp`)
    (set `self.UpdateTextureXLocation` _locationx)
    (set `self.UpdateTextureYLocation` _locationy)
    (`self.DrawTextureSimple` (`/Game/Blueprints/Pickups/BaseItemPlaceHolder.ItemInventoryTexture` (`self.Item Being Moved`)) (`self.UpdateTextureXLocation`) (`self.UpdateTextureYLocation`))))

(fn `UserConstructionScript`)