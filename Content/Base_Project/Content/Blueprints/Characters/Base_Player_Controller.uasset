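; Base player controller that turns movement and look axis inputs into motion of player character 0.
; Forward and strafe axes add movement input along directions built from control rotation yaw only, so camera pitch does not affect movement.
; Mouse and gamepad look axes feed controller yaw and pitch input directly, with no sensitivity or delta-time scaling.
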(event `InputAxis|MoveForwardBackward`
  (params (AxisValue :type "Float (single-precision)"))
  ;[0.1839 0.7674 1 0.206] Input
  ;;[1 0 0 0.457] Movement
  (`Pawn.AddMovementInput` (`GameplayStatics.GetPlayerCharacter` 0) (`KismetMathLibrary.GetForwardVector` (`KismetMathLibrary.MakeRot` 0.0 (.yaw (`self.GetControlRotation`)))) AxisValue))

(event `InputAxis|StrafeLeftRight`
  (params (AxisValue :type "Float (single-precision)"))
  ;[0.1839 0.7674 1 0.206] Input
  ;;[1 0 0 0.457] Movement
  (`Pawn.AddMovementInput` (`GameplayStatics.GetPlayerCharacter` 0) (`KismetMathLibrary.GetRightVector` (`KismetMathLibrary.MakeRot` 0.0 (.yaw (`self.GetControlRotation`)))) AxisValue))

(event `InputAxis|MouseLookLeftRight`
  (params (AxisValue :type "Float (single-precision)"))
  ;[0.1839 0.7674 1 0.206] Input
  ;;[0 0.04714 1 0.229] Look
  (`Pawn.AddControllerYawInput` (`GameplayStatics.GetPlayerCharacter` 0) AxisValue))

(event `InputAxis|MouseLookUpDown`
  (params (AxisValue :type "Float (single-precision)"))
  ;[0.1839 0.7674 1 0.206] Input
  ;;[0 0.04714 1 0.229] Look
  (`Pawn.AddControllerPitchInput` (`GameplayStatics.GetPlayerCharacter` 0) AxisValue))

(event `InputAxis|GamePadLookUpDown`
  (params (AxisValue :type "Float (single-precision)"))
  ;[0.1839 0.7674 1 0.206] Input
  ;;[0 0.04714 1 0.229] Look
  (`Pawn.AddControllerPitchInput` (`GameplayStatics.GetPlayerCharacter` 0) AxisValue))

(event `InputAxis|GamePadLookLeftRight`
  (params (AxisValue :type "Float (single-precision)"))
  ;[0.1839 0.7674 1 0.206] Input
  ;;[0 0.04714 1 0.229] Look
  (`Pawn.AddControllerYawInput` (`GameplayStatics.GetPlayerCharacter` 0) AxisValue))

(fn `UserConstructionScript`)