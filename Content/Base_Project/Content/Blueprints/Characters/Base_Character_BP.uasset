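; Base character with first/third-person camera zoom, a top-down minimap camera, a mouse-cursor mode toggle and a slot-based item inventory.
; The mouse wheel adjusts boom length or FOV and switches view modes at the limits.
; Pickup traces from the camera, then repeats under authority to send and destroy the world item.
; Authority-gated events spawn items into the first empty slot and update slots from HUD hit-box indices.
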(event `self.ReceiveTick`
  (params (DeltaSeconds :type "Float (single-precision)"))
  (`SceneComponent.SetRelativeRotation` (`self.MiniMap Camera`) (`KismetMathLibrary.MakeRot` (`KismetMathLibrary.ClampAngle` (.pitch (`SceneComponent.RelativeRotation` (`self.MiniMap Camera`))) -90.0 -90.0) (`KismetMathLibrary.ClampAngle` (.yaw (`SceneComponent.RelativeRotation` (`self.MiniMap Camera`))) 0.0 0.0) (`KismetMathLibrary.ClampAngle` (.roll (`SceneComponent.RelativeRotation` (`self.MiniMap Camera`))) 0.0 0.0)) false))

(event `self.ReceiveBeginPlay`
  ;[1 1 1] Initialising
  (`KismetArrayLibrary.Array_Resize` (`self.CharacterInventory`) (`self.Inventory slots`)))

(event `InputAction|Action`
  ;[1 1 1] local raycast call to server
  (:`Pressed`
    (bind (_trace_hit _hit_object_actor) (`self.ActorTraceHitCheck`))
    (if _trace_hit
      (`/Engine/EditorBlueprintResources/StandardMacros.IsValid` _hit_object_actor
        (:`Is Valid`
          (`self.ItemPickedUp`))))))

(event `InputAction|ToggleCamera`
  ;[1 1 1] Input
  ;;[0.095 0.095 0.095] Camera Control
  (:`Pressed`
    (`self.Toggle Camera`)))

(event `Key|MouseScrollDown`
  ;[1 1 1] Input
  ;;[0.095 0.095 0.095] Camera Control
  (:`Pressed`
    (`self.Camera Wheel Down`)))

(event `ItemPickedUp`
  ;[1 1 1] server check for actor hit and destroy world actor
  (`/Engine/EditorBlueprintResources/ActorMacros.Switch Has Authority`
    (:`Authority`
      (bind _returninventoryamount (`self.CheckIfInventoryIsFull`))
      (if (not _returninventoryamount)
        (`self.ServerCheckHitTrace` self)))))

(event `Key|MouseScrollUp`
  ;[1 1 1] Input
  ;;[0.095 0.095 0.095] Camera Control
  (:`Pressed`
    (`self.Camera Wheel Up`)))

(event `SendDestroyItemFromLocal`
  (params (ItemIn :type "Actor Object Reference"))
  ;[1 1 1] Send Item from character
  (bind _asbaseitemplaceholder_c (cast `/Game/Blueprints/Pickups/BaseItemPlaceHolder` ItemIn))
  (`/Game/Blueprints/Pickups/BaseItemPlaceHolder.SendItem` _asbaseitemplaceholder_c self))

(event `UpdateinventoryItemsViaHud`
  ;[1 1 1] Switchin/ adding and moving items in the inventory
  (`/Engine/EditorBlueprintResources/ActorMacros.Switch Has Authority`
    (:`Authority`
      (`self.DetermineHitBox`))))

(event `InputAction|Mouse Input`
  (bind _returnvalue (`GameplayStatics.GetPlayerController` 0))
  ;[1 1 1] Input
  ;;[1 1 1] toggle mouse control
  (:`Pressed`
    (`/Engine/EditorBlueprintResources/StandardMacros.FlipFlop`
      (:`A`
        (set `self.Is Input Mode` true)
        (set `PlayerController.bShowMouseCursor` true _returnvalue)
        (set `PlayerController.bEnableClickEvents` true _returnvalue)
        (set `PlayerController.bEnableMouseOverEvents` true _returnvalue)
        (`PlayerController.SetIgnoreMoveInput` _returnvalue true)
        (`PlayerController.SetIgnoreLookInput` _returnvalue true))
      (:`B`
        (set `self.Is Input Mode` false)
        (set `PlayerController.bShowMouseCursor` false _returnvalue)
        (set `PlayerController.bEnableClickEvents` false _returnvalue)
        (set `PlayerController.bEnableMouseOverEvents` false _returnvalue)
        (`PlayerController.SetIgnoreMoveInput` _returnvalue false)
        (`PlayerController.SetIgnoreLookInput` _returnvalue false)))))

(event `DetermineHitBox`
  ;[1 1 1] Switchin/ adding and moving items in the inventory
  (bind (_button_pressed _button_highlighted) (`self.GetHitBoxInfoFromHud`))
  (`self.UpdateHitBoxInfo` _button_pressed _button_highlighted))

(event `PlaceItemInInventory`
  (params (`Inventory Class` :type "Actor Class Reference") (`Assigned Texture` :type "Texture2D Object Reference") (`PickUp Class` :type "Actor Class Reference"))
  ;[1 1 1] Place the item into inventory
  (`/Engine/EditorBlueprintResources/ActorMacros.Switch Has Authority`
    (:`Authority`
      (`self.AddItem` `Inventory Class` `Assigned Texture` `PickUp Class`))))

(event `UpdateHitBoxInfo`
  (params (`Button Pressed` :type Integer) (`Button Highlighted` :type Integer))
  ;[1 1 1] Switchin/ adding and moving items in the inventory
  (`self.SwitchItemInInventory` `Button Pressed` `Button Highlighted`))

(fn `ActorTraceHitCheck`
  (returns (`Trace Hit` :type Boolean) (`Hit Object Actor` :type "Actor Object Reference"))
  (bind _thirdpersoncamera (`self.ThirdPersonCamera`))
  (bind _returnvalue (`SceneComponent.K2_GetComponentLocation` _thirdpersoncamera))
  (bind (_outhit _returnvalue_2) (`KismetSystemLibrary.LineTraceSingle` :`Start` _returnvalue :`End` (+ _returnvalue (* (`SceneComponent.GetForwardVector` _thirdpersoncamera) (`self.CharacterPickupDetectionDist`))) :`TraceChannel` "TraceTypeQuery2" :`DrawDebugType` "Persistent"))
  (return _returnvalue_2 (`.HitActor` (`GameplayStatics.BreakHitResult` _outhit))))

(fn `AddItem`
  (params (`Inventory Class` :type "Actor Class Reference") (TextureToAssign :type "Texture2D Object Reference") (`PickUp Class` :type "Actor Class Reference"))
  (bind _characterinventory (`self.CharacterInventory`))
  (bind _currentinventoryamount (`self.CurrentInventoryAmount`))
  (if (>= (`self.CurrentInventoryAmount`) (`self.MaxInventoryAmount`))
    (`KismetSystemLibrary.PrintString` "Inventory Full")
    (else
      (bind _returnvalue (`|SpawnActorFromClass` `Inventory Class` (`KismetMathLibrary.MakeTransform` (0.0 0.0 0.0))))
      (bind _asbaseitemplaceholder_c (cast `/Game/Blueprints/Pickups/BaseItemPlaceHolder` _returnvalue))
      (for (_array_element _array_index) _characterinventory
        (`/Engine/EditorBlueprintResources/StandardMacros.IsValid` _array_element
          (:`Is Not Valid`
            (`KismetArrayLibrary.Array_Set` _characterinventory _array_index _asbaseitemplaceholder_c)
            (set `/Game/Blueprints/Pickups/BaseItemPlaceHolder.ItemInventoryTexture` TextureToAssign _asbaseitemplaceholder_c)
            (set `/Game/Blueprints/Pickups/BaseItemPlaceHolder.Pick Up Class` `PickUp Class` _asbaseitemplaceholder_c)
            (break))))
      (set `self.CurrentInventoryAmount` (+ _currentinventoryamount 1))
      (`KismetSystemLibrary.PrintString` (`KismetStringLibrary.Concat_StrStr` "current inventory amount" (`KismetStringLibrary.Conv_IntToString` _currentinventoryamount))))))

(fn `Camera Wheel Down`
  (bind _cameraboom (`self.CameraBoom`))
  (bind _thirdpersoncamera (`self.ThirdPersonCamera`))
  (bind _returnvalue (+ (`CameraComponent.FieldOfView` (`self.ThirdPersonCamera`)) (`self.ZoomIncrementAmount`)))
  (bind _returnvalue_2 (+ (`SpringArmComponent.TargetArmLength` _cameraboom) (`self.ZoomIncrementAmount`)))
  (if (`self.IsfirstPerson`)
    ;[1 1 1] Controls the field of view for first person perspective and limits it to a range
    (set `CameraComponent.FieldOfView` (`KismetMathLibrary.FClamp` _returnvalue (`self.MinFoV`) (`self.MaxFoV`)) _thirdpersoncamera)
    (`KismetSystemLibrary.PrintString` (`KismetStringLibrary.Conv_DoubleToString` _returnvalue))
    ;[1 1 1] scrolling in and out of camera modes
    (set `self.IsfirstPerson` (< (`CameraComponent.FieldOfView` _thirdpersoncamera) (`self.MaxFoV`)))
    (else
      ;[1 1 1] Controls the third person perspective and limits it to a range
      (set `SpringArmComponent.TargetArmLength` (`KismetMathLibrary.FClamp` _returnvalue_2 (`self.MinCameraDistance`) (`self.MaxCameraDistance`)) _cameraboom)
      (`KismetSystemLibrary.PrintString` (`KismetStringLibrary.Conv_DoubleToString` _returnvalue_2)))))

(fn `Camera Wheel Up`
  (bind _cameraboom (`self.CameraBoom`))
  (bind _returnvalue (- (`SpringArmComponent.TargetArmLength` _cameraboom) (`self.ZoomIncrementAmount`)))
  (bind _returnvalue_2 (- (`CameraComponent.FieldOfView` (`self.ThirdPersonCamera`)) 10.0))
  (if (`self.IsfirstPerson`)
    (set `CameraComponent.FieldOfView` (`KismetMathLibrary.FClamp` _returnvalue_2 (`self.MinFoV`) (`self.MaxFoV`)) (`self.ThirdPersonCamera`))
    (`KismetSystemLibrary.PrintString` (`KismetStringLibrary.Conv_DoubleToString` _returnvalue_2))
    (else
      (set `SpringArmComponent.TargetArmLength` (`KismetMathLibrary.FClamp` _returnvalue (`self.MinCameraDistance`) (`self.MaxCameraDistance`)) _cameraboom)
      (`KismetSystemLibrary.PrintString` (`KismetStringLibrary.Conv_DoubleToString` _returnvalue))
      ;[1 1 1] scrolling in and out of camera modes
      (set `self.IsfirstPerson` (< (`SpringArmComponent.TargetArmLength` (`self.CameraBoom`)) (+ (`self.MinCameraDistance`) 1.0))))))

(fn `CheckIfInventoryIsFull`
  (returns (ReturnInventoryAmount :type Boolean))
  (return (>= (`self.CurrentInventoryAmount`) (`self.MaxInventoryAmount`))))

(fn `GetHitBoxInfoFromHud`
  (returns (`Button Pressed` :type Integer) (`Button Highlighted` :type Integer))
  (bind _asbase_hud_c (cast `/Game/Blueprints/Hud/Base_HUD` (`PlayerController.GetHUD` (`GameplayStatics.GetPlayerController` 0))))
  (return (`/Game/Blueprints/Hud/Base_HUD.HitBox To Int` _asbase_hud_c) (`/Game/Blueprints/Hud/Base_HUD.HitBoxHighlighted` _asbase_hud_c)))

(fn `ServerCheckHitTrace`
  (params (Character :type "/Game/Blueprints/Characters/Base_Character_BP Object Reference"))
  (`/Engine/EditorBlueprintResources/ActorMacros.Switch Has Authority`
    (:`Authority`
      (bind (_trace_hit _hit_object_actor) (`self.ActorTraceHitCheck`))
      (if _trace_hit
        (`/Engine/EditorBlueprintResources/StandardMacros.IsValid` _hit_object_actor
          (:`Is Valid`
            (`self.SendDestroyItemFromLocal` _hit_object_actor)
            (`self.K2_DestroyActor` _hit_object_actor)))))))

(fn `SwitchItemInInventory`
  (params (`Button Pressed` :type Integer) (`Button Highlighted` :type Integer))
  (bind _characterinventory (`self.CharacterInventory`))
  (if (== `Button Pressed` `Button Highlighted`)
    (bind _asbase_hud_c (cast `/Game/Blueprints/Hud/Base_HUD` (`PlayerController.GetHUD` (`GameplayStatics.GetPlayerController` 0))))
    (`KismetArrayLibrary.Array_Set` _characterinventory `Button Pressed` (`KismetArrayLibrary.Array_Get` _characterinventory `Button Highlighted`))
    (`KismetArrayLibrary.Array_Set` _characterinventory `Button Highlighted` (`/Game/Blueprints/Hud/Base_HUD.Item Being Moved` _asbase_hud_c))))

(fn `Toggle Camera`
  ;[1 1 1] Toggles the camera between First and Third Person while also resetting the camera position
  (if (`self.IsfirstPerson`)
    (set `self.IsfirstPerson` false)
    (set `CameraComponent.FieldOfView` (`self.MaxFoV`) (`self.ThirdPersonCamera`))
    (set `SpringArmComponent.TargetArmLength` (`self.MinCameraDistance`) (`self.CameraBoom`))
    (`KismetSystemLibrary.PrintString` "1st person")
    (else
      (set `self.IsfirstPerson` true)
      (set `SpringArmComponent.TargetArmLength` (`self.MaxCameraDistance`) (`self.CameraBoom`))
      (`KismetSystemLibrary.PrintString` "3rd person"))))

(fn `UserConstructionScript`)