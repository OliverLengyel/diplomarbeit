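; Base weapon Blueprint, still work in progress, with variables for range, damage, area of effect, fire rate and setup.
; Only the range check runs: every Tick it compares GetDistanceTo, with no target actor specified, against min and max range to set WeaponInRange.
; Unconnected draft snippets sketch setup/set-down montages, a forward line trace, a fire-rate delay, random radial damage and a fire-on-move branch.
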(event `self.ReceiveTick`
  (params (DeltaSeconds :type "Float (single-precision)"))
  (`self.WeaponRangeCheck`))

(event `WeaponRangeCheck`
  ;[1 1 1] Wip Script to get weapon max and min range to deal damage.Not what i want to implement.
  (bind _returnvalue (`self.GetDistanceTo` null))
  (if (== (> _returnvalue (`self.Min Weapon Range`)) (<= _returnvalue (`self.Max Weapon Range`)))
    (set `self.WeaponInRange` true)
    (else
      (set `self.WeaponInRange` false))))

(fn `UserConstructionScript`)